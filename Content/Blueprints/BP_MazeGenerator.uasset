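; Generates a random tile maze on BeginPlay and builds it in the level from spawned BP_Wall actors.
; Fills a flat array with walls at odd-adjusted dimensions, then carves paths by iterative randomised depth-first backtracking, using trace arrays as the stack.
; Marks an exit beside a random path tile near the far-X edge before spawning the walls, leaving path and exit tiles empty.
; ResetMaze can refill tiles with walls but is not called here.
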(event EventBeginPlay
  (Utilities|FlowControl|Sequence
    (:then_0
      (CallFunction|Initialise))
    (:then_1
      (CallFunction|InitialiseMaze))
    (:then_2
      (CallFunction|GenerateMaze))
    (:then_3
      (CallFunction|PlaceExit))
    (:then_4
      (CallFunction|DrawMaze))))

(fn ConstructionScript)

(fn Initialise
  (Utilities|FlowControl|Sequence
    (:then_0
      (if (== (Math|Integer|%(Integer) (Variables|Default|GetMAZE_WIDTH) 2) 0)
        (Variables|Default|SetmazeWidth (+ (Variables|Default|GetMAZE_WIDTH) 1))
        (else
          (Variables|Default|SetmazeWidth (Variables|Default|GetMAZE_WIDTH)))))
    (:then_1
      (if (== (Math|Integer|%(Integer) (Variables|Default|GetMAZE_HEIGHT) 2) 0)
        (Variables|Default|SetmazeHeight (+ (Variables|Default|GetMAZE_HEIGHT) 1))
        (else
          (Variables|Default|SetmazeHeight (Variables|Default|GetMAZE_HEIGHT)))))
    (:then_2
      (Variables|Default|Setnodes (- (/ (* (Variables|Default|GetmazeWidth) (Variables|Default|GetmazeHeight)) 4) 1)))))

(fn InitialiseMaze
  (for _index (range 0 (- (* (Variables|Default|GetmazeWidth) (Variables|Default|GetmazeHeight)) 1))
    (Utilities|Array|Add (Variables|Default|GetmazeArray) (Variables|Default|GetWALL))))

(fn SetMazeTile
  (params (mazeTileX :type Integer) (mazeTileY :type Integer) (mazeTile :type Integer))
  (Utilities|Array|SetArrayElem (Variables|Default|GetmazeArray) (+ mazeTileX (* mazeTileY (Variables|Default|GetmazeWidth))) mazeTile))

(fn ReadMazeTile
  (params (mazeTileX :type Integer) (mazeTileY :type Integer))
  (return (Utilities|Array|Get(acopy) (Variables|Default|GetmazeArray) (+ mazeTileX (* mazeTileY (Variables|Default|GetmazeWidth))))))

(fn GenerateMaze
  (Utilities|FlowControl|Sequence
    (:then_0
      (LocalVariables|SetmazePathX (Variables|Default|GetPATH_START_X)))
    (:then_1
      (LocalVariables|SetmazePathY (Variables|Default|GetPATH_START_Y)))
    (:then_2
      (LocalVariables|SetpathLength 0))
    (:then_3
      (for _index (range 0 (- (Variables|Default|Getnodes) 1))
        (Utilities|Array|Add (LocalVariables|GetnewPathDirectionX) 0)))
    (:then_4
      (for _index_2 (range 0 (- (Variables|Default|Getnodes) 1))
        (Utilities|Array|Add (LocalVariables|GetnewPathDirectionY) 0)))
    (:then_5
      (for _index_3 (range 0 (- (Variables|Default|Getnodes) 1))
        (Utilities|Array|Add (LocalVariables|GetpathTraceX) 0)))
    (:then_6
      (for _index_4 (range 0 (- (Variables|Default|Getnodes) 1))
        (Utilities|Array|Add (LocalVariables|GetpathTraceY) 0)))
    (:then_7
      (Utilities|FlowControl|Sequence :!label _label
        (:then_0
          (CallFunction|SetMazeTile (LocalVariables|GetmazePathX) (LocalVariables|GetmazePathY) (Variables|Default|GetPATH)))
        (:then_1
          (LocalVariables|SetpathDirections 0))
        (:then_2
          ;[1 1 1] // mazePathY > 2
          (if (> (LocalVariables|GetmazePathY) 2)
            (bind _mazetile (CallFunction|ReadMazeTile (LocalVariables|GetmazePathX) (- (LocalVariables|GetmazePathY) 2)))
            (LocalVariables|SettileType _mazetile)
            (if (== (LocalVariables|GettileType) (Variables|Default|GetWALL))
              (Utilities|FlowControl|Sequence
                (:then_0
                  (Utilities|Array|SetArrayElem (LocalVariables|GetnewPathDirectionX) (LocalVariables|GetpathDirections) 0))
                (:then_1
                  (Utilities|Array|SetArrayElem (LocalVariables|GetnewPathDirectionY) (LocalVariables|GetpathDirections) (Variables|Default|GetDOWN)))
                (:then_2
                  (LocalVariables|SetpathDirections (+ (LocalVariables|GetpathDirections) 1)))
                (:then_3
                  ;[1 1 1] // mazePathX < mazeWidth - 2
                  (if (< (LocalVariables|GetmazePathX) (- (Variables|Default|GetmazeWidth) 2)) :!label _label_2
                    (bind _mazetile_2 (CallFunction|ReadMazeTile (+ (LocalVariables|GetmazePathX) 2) (LocalVariables|GetmazePathY)))
                    (LocalVariables|SettileType _mazetile_2)
                    (if (== (LocalVariables|GettileType) (Variables|Default|GetWALL))
                      (Utilities|FlowControl|Sequence
                        (:then_0
                          (Utilities|Array|SetArrayElem (LocalVariables|GetnewPathDirectionX) (LocalVariables|GetpathDirections) (Variables|Default|GetRIGHT)))
                        (:then_1
                          (Utilities|Array|SetArrayElem (LocalVariables|GetnewPathDirectionY) (LocalVariables|GetpathDirections) 0))
                        (:then_2
                          (LocalVariables|SetpathDirections (+ (LocalVariables|GetpathDirections) 1)))
                        (:then_3
                          ;[1 1 1] // mazePathY < mazeHeight - 2
                          (if (< (LocalVariables|GetmazePathY) (- (Variables|Default|GetmazeHeight) 2)) :!label _label_3
                            (bind _mazetile_3 (CallFunction|ReadMazeTile (LocalVariables|GetmazePathX) (+ (LocalVariables|GetmazePathY) 2)))
                            (LocalVariables|SettileType _mazetile_3)
                            (if (== (LocalVariables|GettileType) (Variables|Default|GetWALL))
                              (Utilities|FlowControl|Sequence
                                (:then_0
                                  (Utilities|Array|SetArrayElem (LocalVariables|GetnewPathDirectionX) (LocalVariables|GetpathDirections) 0))
                                (:then_1
                                  (Utilities|Array|SetArrayElem (LocalVariables|GetnewPathDirectionY) (LocalVariables|GetpathDirections) (Variables|Default|GetUP)))
                                (:then_2
                                  (LocalVariables|SetpathDirections (+ (LocalVariables|GetpathDirections) 1)))
                                (:then_3
                                  ;[1 1 1] // mazePathX > 2
                                  (if (> (LocalVariables|GetmazePathX) 2) :!label _label_4
                                    (bind _mazetile_4 (CallFunction|ReadMazeTile (- (LocalVariables|GetmazePathX) 2) (LocalVariables|GetmazePathY)))
                                    (LocalVariables|SettileType _mazetile_4)
                                    (if (== (LocalVariables|GettileType) (Variables|Default|GetWALL))
                                      (Utilities|FlowControl|Sequence
                                        (:then_0
                                          (Utilities|Array|SetArrayElem (LocalVariables|GetnewPathDirectionX) (LocalVariables|GetpathDirections) (Variables|Default|GetLEFT)))
                                        (:then_1
                                          (Utilities|Array|SetArrayElem (LocalVariables|GetnewPathDirectionY) (LocalVariables|GetpathDirections) 0))
                                        (:then_2
                                          (LocalVariables|SetpathDirections (+ (LocalVariables|GetpathDirections) 1)))
                                        (:then_3
                                          ;[1 1 1] // if pathDirections == 0
                                          (if (== (LocalVariables|GetpathDirections) 0) :!label _label_5
                                            ;[1 1 1] // if pathLength > 0
                                            (if (> (LocalVariables|GetpathLength) 0)
                                              ;[1 1 1] // for loop
                                              (LocalVariables|SetpathSearch (- (LocalVariables|GetpathLength) 1))
                                              (if (> (LocalVariables|GetpathSearch) 0) :!label _label_6
                                                (if (and (== (Utilities|Array|Get(acopy) (LocalVariables|GetpathTraceX) (LocalVariables|GetpathSearch)) (LocalVariables|GetmazePathX)) (== (Utilities|Array|Get(acopy) (LocalVariables|GetpathTraceY) (LocalVariables|GetpathSearch)) (LocalVariables|GetmazePathY)))
                                                  (Utilities|FlowControl|Sequence
                                                    (:then_0
                                                      (Utilities|Array|SetArrayElem (LocalVariables|GetpathTraceX) (LocalVariables|GetpathSearch) 0))
                                                    (:then_1
                                                      (Utilities|Array|SetArrayElem (LocalVariables|GetpathTraceY) (LocalVariables|GetpathSearch) 0))
                                                    (:then_2
                                                      (LocalVariables|SetpathSearch (- (LocalVariables|GetpathSearch) 1) :!label _label_7)
                                                      (goto _label_6)))
                                                  (else
                                                    (goto _label_7)))
                                                (else
                                                  (LocalVariables|SetpathLength (- (LocalVariables|GetpathLength) 1))
                                                  (if (!= (LocalVariables|GetpathDirections) 0) :!label _label_8
                                                    (goto _label)
                                                    (else
                                                      ;[1 1 1] // if pathLength > 0
                                                      (if (> (LocalVariables|GetpathLength) 0)
                                                        (Utilities|FlowControl|Sequence
                                                          (:then_0
                                                            (LocalVariables|SetmazePathX (Utilities|Array|Get(acopy) (LocalVariables|GetpathTraceX) (- (LocalVariables|GetpathLength) 1))))
                                                          (:then_1
                                                            (LocalVariables|SetmazePathY (Utilities|Array|Get(acopy) (LocalVariables|GetpathTraceY) (- (LocalVariables|GetpathLength) 1))))
                                                          (:then_2
                                                            (if (!= (LocalVariables|GetpathLength) 0) :!label _label_9
                                                              (goto _label)
                                                              (else
                                                                (Development|PrintString "Maze complete . . ." true true "(R=0.000000,G=0.660000,B=1.000000,A=1.000000)" 1e+01)))))
                                                        (else
                                                          (goto _label_9)))))))
                                              (else
                                                (goto _label_8)))
                                            (else
                                              (Utilities|FlowControl|Sequence ; // else
                                                (:then_0
                                                  (LocalVariables|SetrandomPathDirection (Math|Random|RandomIntegerinRange 0 (- (LocalVariables|GetpathDirections) 1))))
                                                (:then_1
                                                  (LocalVariables|SetrandomPathCellX (+ (LocalVariables|GetmazePathX) (Utilities|Array|Get(acopy) (LocalVariables|GetnewPathDirectionX) (LocalVariables|GetrandomPathDirection)))))
                                                (:then_2
                                                  (LocalVariables|SetrandomPathCellY (+ (LocalVariables|GetmazePathY) (Utilities|Array|Get(acopy) (LocalVariables|GetnewPathDirectionY) (LocalVariables|GetrandomPathDirection)))))
                                                (:then_3
                                                  (CallFunction|SetMazeTile (LocalVariables|GetrandomPathCellX) (LocalVariables|GetrandomPathCellY) (Variables|Default|GetPATH)))
                                                (:then_4
                                                  (LocalVariables|SetmazePathX (+ (LocalVariables|GetmazePathX) (* (Utilities|Array|Get(acopy) (LocalVariables|GetnewPathDirectionX) (LocalVariables|GetrandomPathDirection)) 2))))
                                                (:then_5
                                                  (LocalVariables|SetmazePathY (+ (LocalVariables|GetmazePathY) (* (Utilities|Array|Get(acopy) (LocalVariables|GetnewPathDirectionY) (LocalVariables|GetrandomPathDirection)) 2))))
                                                (:then_6
                                                  (Utilities|Array|SetArrayElem (LocalVariables|GetpathTraceX) (LocalVariables|GetpathLength) (LocalVariables|GetmazePathX)))
                                                (:then_7
                                                  (Utilities|Array|SetArrayElem (LocalVariables|GetpathTraceY) (LocalVariables|GetpathLength) (LocalVariables|GetmazePathY)))
                                                (:then_8
                                                  (LocalVariables|SetpathLength (+ (LocalVariables|GetpathLength) 1)))
                                                (:then_9
                                                  (goto _label_8)))))))
                                      (else
                                        (goto _label_5)))
                                    (else
                                      (goto _label_5)))))
                              (else
                                (goto _label_4)))
                            (else
                              (goto _label_4)))))
                      (else
                        (goto _label_3)))
                    (else
                      (goto _label_3)))))
              (else
                (goto _label_2)))
            (else
              (goto _label_2))))))))

(fn DrawMaze
  (for _index (range 0 (- (Variables|Default|GetMAZE_HEIGHT) 1))
    (for _index_2 (range 0 (- (Variables|Default|GetMAZE_WIDTH) 1))
      (bind _output_get (LocalVariables|SetcellX _index_2))
      (bind _output_get_2 (LocalVariables|SetcellY _index))
      (bind _mazetile (CallFunction|ReadMazeTile _output_get _output_get_2))
      (if (== _mazetile (Variables|Default|GetWALL))
        (bind _result (Math|Float|NegateFloat (Math|Conversions|ToFloat(Integer) (* (LocalVariables|GetcellY) (Variables|Default|GetTILE_HEIGHT))))
          (:%20%20
            (Game|SpawnActorfromClass "/Game/Blueprints/BP_Wall.BP_Wall_C" (Math|Transform|MakeTransform (Math|Vector|MakeVector (Math|Conversions|ToFloat(Integer) (* (LocalVariables|GetcellX) (Variables|Default|GetTILE_WIDTH))) _result (Math|Conversions|ToFloat(Integer) (/ (Variables|Default|GetTILE_HEIGHT) 2))) "0, 0, 0" "1,1,1") "Undefined" 0 0)))))))

(fn ResetMaze
  (for _index (range (LocalVariables|GettileY) (Variables|Default|GetmazeHeight))
    (for _index_2 (range (LocalVariables|GettileX) (Variables|Default|GetmazeWidth))
      (CallFunction|SetMazeTile _index_2 _index (Variables|Default|GetWALL)))))

(fn PlaceExit
  (LocalVariables|SetexitPositionX (- (Variables|Default|GetMAZE_WIDTH) 2))
  (LocalVariables|SetexitPositionY (Math|Random|RandomIntegerinRange (Variables|Default|GetMINIMUM_EXIT_POSITION_Y) (- (Variables|Default|GetMAZE_HEIGHT) 1)) :!label _label)
  (bind _mazetile (CallFunction|ReadMazeTile (LocalVariables|GetexitPositionX) (LocalVariables|GetexitPositionY)))
  (LocalVariables|SettileType _mazetile)
  (if (== (LocalVariables|GettileType) (Variables|Default|GetPATH))
    (CallFunction|SetMazeTile (+ (LocalVariables|GetexitPositionX) 1) (LocalVariables|GetexitPositionY) (Variables|Default|GetEXIT))
    (else
      (goto _label))))